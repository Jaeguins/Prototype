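; Blueprint function library that provides global accessors for the VP framework's core objects: VPInitManager, EXP_EditManager and VPGameInstance.
; The two manager getters find their actor by class and "Module" tag, while the game instance getter reads the current GameInstance.
; Each getter validates and casts the result, reporting invalid objects or failed casts through Korean-language log or print messages.
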(fn `GetEditManager`
  (returns (VPEditManager :type "/Game/Prototype/Module/Edit/EXP_EditManager Object Reference"))
  (bind _returnvalue (`MinusiFrameworkLibrary.GetSpecificFirstActorWithTag` null "Module" "/Game/Prototype/Module/Edit/EXP_EditManager.EXP_EditManager_C"))
  (`/Engine/EditorBlueprintResources/StandardMacros.IsValid` _returnvalue
    (:`Is Valid`
      (bind _asexp_edit_manager (cast `/Game/Prototype/Module/Edit/EXP_EditManager` _returnvalue)
        (:`then`
          (return _asexp_edit_manager))
        (:`CastFailed`
          (`KismetSystemLibrary.PrintString` null "VPLib :: EditManager로의 캐스팅이 유효하지 않습니다 :: GetEditManager"))))
    (:`Is Not Valid`
      (`MinusiFrameworkLibrary.ScreenLongLog` "VPLib :: EditManager가 유효하지 않습니다."))))

(fn `GetInitInstance`
  (returns (InitInstance :type "/Game/Blueprint/Module/Init/VPInitManager Object Reference"))
  (bind _returnvalue (`MinusiFrameworkLibrary.GetSpecificFirstActorWithTag` null "Module" "/Game/Blueprint/Module/Init/VPInitManager.VPInitManager_C"))
  (`/Engine/EditorBlueprintResources/StandardMacros.IsValid` _returnvalue
    (:`Is Valid`
      (bind _asvpinit_manager (cast `/Game/Blueprint/Module/Init/VPInitManager` _returnvalue)
        (:`then`
          (return _asvpinit_manager))
        (:`CastFailed`
          (`KismetSystemLibrary.PrintString` null "VPLib :: InitManager로의 캐스팅이 유효하지 않습니다 :: GetInitInstance"))))
    (:`Is Not Valid`
      (`MinusiFrameworkLibrary.ScreenLongLog` "VPLib :: InitManager가 유효하지 않습니다."))))

(fn `GetVPGameInstance`
  (returns (`VPGame Instance` :type "VPGameInstance Object Reference"))
  (bind _returnvalue (`GameplayStatics.GetGameInstance` null))
  (`/Engine/EditorBlueprintResources/StandardMacros.IsValid` _returnvalue
    (:`Is Valid`
      (bind _asvpgame_instance (cast `VPGameInstance` _returnvalue)
        (:`then`
          (return _asvpgame_instance))
        (:`CastFailed`
          (`KismetSystemLibrary.PrintString` null "VPLib :: VPGameInstance로의 캐스팅이 유효하지 않습니다 :: GetGameInstance"))))
    (:`Is Not Valid`
      (`MinusiFrameworkLibrary.ScreenLongLog` "VPLib :: GameInstance가 유효하지 않습니다."))))